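; Inventory actor component that stores picked-up items in eight slots and toggles the WB_Inventario widget with IA_Inventario, switching cursor, input mode and look input.
; AgarrarObjeto tops up matching partial stacks, then fills empty slots, returning any quantity that does not fit.
; AgregarASlot caps each stack at CantidadMaxima and refreshes the widget after every write.
; Stackable items never land in slot 0, because their index checks use > 0.
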(event Input|EnhancedActionEvents|EnhancedInputActionIA_Inventario
  (params (ActionValue :type Boolean) (ElapsedSeconds :type Float%20%28double-precision%29) (TriggeredSeconds :type Float%20%28double-precision%29) (InputAction :type Input%20Action%20Object%20Reference :default "/Game/FirstPerson/Input/Actions/IA_Inventario.IA_Inventario"))
  (bind _returnvalue (Game|GetPlayerController 0))
  (:Started
    (if (Widget|IsVisible (Variables|Default|GetWidget%20Inventario))
      (Variables|/Script/Engine.PlayerController|SetbShowMouseCursor _returnvalue false)
      (Widget|RemovefromParent (Variables|Default|GetWidget%20Inventario))
      (Input|SetInputModeGameOnly _returnvalue false)
      (Input|ResetIgnoreLookInput _returnvalue)
      (else
        (Variables|/Script/Engine.PlayerController|SetbShowMouseCursor _returnvalue true)
        (Input|SetInputModeGameandUI _returnvalue 0 "DoNotLock" true false)
        (UserInterface|Viewport|AddtoViewport (Variables|Default|GetWidget%20Inventario) 0)
        (Input|SetIgnoreLookInput _returnvalue true)))))

(event EventBeginPlay
  (bind _returnvalue (UserInterface|CreateWidget "/Game/Inventario/Widgets/WB_Inventario.WB_Inventario_C"))
  (Variables|Default|SetWidget%20Inventario _returnvalue)
  (Utilities|Array|Resize (Variables|Default|GetObjetos) 8)
  (Default|CargarInventario (Variables|Default|GetWidget%20Inventario) self))

(fn AgarrarObjeto
  (params (Objeto :type S%20Objeto%20Structure))
  (LocalVariables|SetNuevo%20Objeto Objeto)
  (if (> (.cantidadmaxima (LocalVariables|GetNuevo%20Objeto)) 1)
    (while (> (.cantidad (LocalVariables|GetNuevo%20Objeto)) 0)
      (bind _pos_slot_libre (CallFunction|BuscarEnElInventario (LocalVariables|GetNuevo%20Objeto)))
      (if (> _pos_slot_libre 0)
        (bind _sobrante (CallFunction|AgregarASlot _pos_slot_libre (LocalVariables|GetNuevo%20Objeto)))
        (LocalVariables|SetNuevo%20Objeto (Utilities|Struct|MakeS_Objeto (.Name (Utilities|Struct|BreakS_Objeto (LocalVariables|GetNuevo%20Objeto))) (.Descripcion (Utilities|Struct|BreakS_Objeto (LocalVariables|GetNuevo%20Objeto))) _sobrante (.CantidadMaxima (Utilities|Struct|BreakS_Objeto (LocalVariables|GetNuevo%20Objeto))) (.Icono (Utilities|Struct|BreakS_Objeto (LocalVariables|GetNuevo%20Objeto))) (.Mesh (Utilities|Struct|BreakS_Objeto (LocalVariables|GetNuevo%20Objeto))) (.Peso (Utilities|Struct|BreakS_Objeto (LocalVariables|GetNuevo%20Objeto))) false))
        (else
          (bind _pos_slot_libre_2 (CallFunction|BuscarSlotLibre))
          (if (> _pos_slot_libre_2 0)
            (bind _sobrante_2 (CallFunction|AgregarASlot _pos_slot_libre_2 (LocalVariables|GetNuevo%20Objeto)))
            (LocalVariables|SetNuevo%20Objeto (Utilities|Struct|MakeS_Objeto (.Name (Utilities|Struct|BreakS_Objeto (LocalVariables|GetNuevo%20Objeto))) (.Descripcion (Utilities|Struct|BreakS_Objeto (LocalVariables|GetNuevo%20Objeto))) _sobrante_2 (.CantidadMaxima (Utilities|Struct|BreakS_Objeto (LocalVariables|GetNuevo%20Objeto))) (.Icono (Utilities|Struct|BreakS_Objeto (LocalVariables|GetNuevo%20Objeto))) (.Mesh (Utilities|Struct|BreakS_Objeto (LocalVariables|GetNuevo%20Objeto))) (.Peso (Utilities|Struct|BreakS_Objeto (LocalVariables|GetNuevo%20Objeto)))))
            (else
              (return (.cantidad (LocalVariables|GetNuevo%20Objeto))))))))
    (return 0)
    (else
      (bind _pos_slot_libre_3 (CallFunction|BuscarSlotLibre))
      (if (>= _pos_slot_libre_3 0)
        (CallFunction|AgregarASlot _pos_slot_libre_3 (LocalVariables|GetNuevo%20Objeto))
        (else
          (return (.cantidad (LocalVariables|GetNuevo%20Objeto))))))))

(fn BuscarEnElInventario
  (params (Objeto :type S%20Objeto%20Structure))
  (LocalVariables|SetNuevo%20Objeto Objeto)
  (for (_array_element _array_index) (Variables|Default|GetObjetos)
    (if (Utilities|Enum|Equal(Enum) (.Name (Utilities|Struct|BreakS_Objeto _array_element)) (.name (LocalVariables|GetNuevo%20Objeto)))
      (if (not (>= (.Cantidad (Utilities|Struct|BreakS_Objeto _array_element)) (.cantidadmaxima (LocalVariables|GetNuevo%20Objeto))))
        (return _array_index))))
  (return -1))

(fn BuscarSlotLibre
  (for (_array_element _array_index) (Variables|Default|GetObjetos)
    (if (Utilities|Enum|Equal(Enum) (.Name (Utilities|Struct|BreakS_Objeto _array_element)) "")
      (return _array_index)))
  (return -1))

(fn AgregarASlot
  (params (Slot :type Integer) (Objeto :type S%20Objeto%20Structure))
  (LocalVariables|SetPos%20Slot Slot)
  (LocalVariables|SetNuevo%20Objeto Objeto)
  (LocalVariables|SetObjeto%20Almacenado (Utilities|Array|Get(acopy) (Variables|Default|GetObjetos) (LocalVariables|GetPos%20Slot)))
  (if (> (+ (.cantidad (LocalVariables|GetObjeto%20Almacenado)) (.cantidad (LocalVariables|GetNuevo%20Objeto))) (.cantidadmaxima (LocalVariables|GetNuevo%20Objeto)))
    (Utilities|Array|SetArrayElem (Variables|Default|GetObjetos) (LocalVariables|GetPos%20Slot) (Utilities|Struct|MakeS_Objeto (.name (LocalVariables|GetNuevo%20Objeto)) (.descripcion (LocalVariables|GetNuevo%20Objeto)) (.cantidadmaxima (LocalVariables|GetNuevo%20Objeto)) (.cantidadmaxima (LocalVariables|GetNuevo%20Objeto)) (.icono (LocalVariables|GetNuevo%20Objeto)) (.mesh (LocalVariables|GetNuevo%20Objeto)) (.peso (LocalVariables|GetNuevo%20Objeto))))
    (Default|CargarInventario (Variables|Default|GetWidget%20Inventario) self)
    (return (- (+ (.cantidad (LocalVariables|GetObjeto%20Almacenado)) (.cantidad (LocalVariables|GetNuevo%20Objeto))) (.cantidadmaxima (LocalVariables|GetNuevo%20Objeto))))
    (else
      (Utilities|Array|SetArrayElem (Variables|Default|GetObjetos) (LocalVariables|GetPos%20Slot) (Utilities|Struct|MakeS_Objeto (.name (LocalVariables|GetNuevo%20Objeto)) (.descripcion (LocalVariables|GetNuevo%20Objeto)) (+ (.cantidad (LocalVariables|GetObjeto%20Almacenado)) (.cantidad (LocalVariables|GetNuevo%20Objeto))) (.cantidadmaxima (LocalVariables|GetNuevo%20Objeto)) (.icono (LocalVariables|GetNuevo%20Objeto)) (.mesh (LocalVariables|GetNuevo%20Objeto)) (.peso (LocalVariables|GetNuevo%20Objeto))))
      (Default|CargarInventario (Variables|Default|GetWidget%20Inventario) self)
      (return 0))))